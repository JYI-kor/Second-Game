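; BP_PlayerState tracks the player's hit points in the GetCoinGame, handling damage, healing and revival.
; BeginPlay revives to MaxHP, and every HP change fires an update dispatcher with current and max HP.
; Damage and healing are ignored once dead, which requires HP strictly below zero.
; Healing clamps to a hard-coded 100 rather than MaxHP, while damage is unclamped.
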(event EventBeginPlay
  (CallFunction|DoRevivePlayerState))

(fn ConstructionScript)

(fn AddDamage
  (params (Damage :type Float%20%28double-precision%29))
  (if (not (CallFunction|IsDeath))
    (Variables|Default|SetCurrent%20HP (- (Variables|Default|GetCurrent%20HP) Damage))
    (Default|CallNewEventDispatcherUpdateHP (Variables|Default|GetCurrent%20HP) (Variables|Default|GetMax%20HP))))

(fn IsDeath
  (return (< (Variables|Default|GetCurrent%20HP) 0.0)))

(fn DoRevivePlayerState
  (Variables|Default|SetCurrent%20HP (Variables|Default|GetMax%20HP))
  (Default|CallNewEventDispatcherUpdateHP (Variables|Default|GetCurrent%20HP) (Variables|Default|GetMax%20HP)))

(fn HealHP
  (params (Heal :type Float%20%28double-precision%29))
  (if (not (CallFunction|IsDeath))
    (Variables|Default|SetCurrent%20HP (Math|Float|Clamp(Float) (+ Heal (Variables|Default|GetCurrent%20HP)) 0.0 1e+02))
    (Default|CallNewEventDispatcherUpdateHP (Variables|Default|GetCurrent%20HP) (Variables|Default|GetMax%20HP))))