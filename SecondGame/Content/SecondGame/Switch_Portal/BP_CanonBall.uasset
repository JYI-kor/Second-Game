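; BP_CanonBall is a cannonball projectile that damages and knocks down player characters it hits.
; On BeginPlay it launches itself with a single forward physics impulse, then destroys itself after a short delay.
; On a component hit against a BP_Graion01Character, it adds fixed damage through that character's BP_PlayerState and switches the character to ragdoll.
; Hits do not destroy the ball, so only the timer ends its life.
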(event OnComponentHit(CanonBall)
  (params (HitComponent :type Primitive%20Component%20Object%20Reference) (OtherActor :type Actor%20Object%20Reference) (OtherComp :type Primitive%20Component%20Object%20Reference) (NormalImpulse :type Vector :default "0, 0, 0") (Hit :type Hit%20Result%20Structure%20%28by%20ref%29))
  (CallFunction|DoHitDamage OtherActor)
  (bind _asbp_graion_01character (Utilities|Casting|CastToBP_Graion01Character OtherActor))
  (Default|DoRagDoll _asbp_graion_01character true))

(event EventBeginPlay
  (bind _canonball (Variables|Default|GetCanonBall))
  (Physics|AddImpulse _canonball (* (Math|Vector|GetForwardVector _canonball) 5e+04) "None" false)
  (Utilities|FlowControl|Delay 2.0)
  (Actor|DestroyActor))

(fn ConstructionScript)

(fn DoHitDamage
  (params (Object :type Object%20Object%20Reference))
  (bind _asbp_graion_01character (Utilities|Casting|CastToBP_Graion01Character Object))
  (bind _asbp_player_state (Utilities|Casting|CastToBP_PlayerState (Variables|/Script/Engine.Pawn|GetPlayerState _asbp_graion_01character)))
  (Default|AddDamage _asbp_player_state 1e+01))